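; BP_ExitDoor is an extraction point that ends a run when the third-person character enters its ExitBox.
; It starts hidden without collision until ShowExitDoor is called to reveal and enable it.
; ExitType selects helicopter extraction, which deducts ExtractionCost from the character's Gold, or free seaport extraction.
; Success calls the character's ShowResult, while insufficient gold prints a message with a hardcoded price.
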(event OnComponentBeginOverlap(ExitBox)
  (params (OverlappedComponent :type Primitive%20Component%20Object%20Reference) (OtherActor :type Actor%20Object%20Reference) (OtherComp :type Primitive%20Component%20Object%20Reference) (OtherBodyIndex :type Integer) (bFromSweep :type Boolean) (SweepResult :type Hit%20Result%20Structure%20%28by%20ref%29))
  (bind _asbp_third_person_character (Utilities|Casting|CastToBP_ThirdPersonCharacter OtherActor))
  (if (== (Variables|Default|GetExitType) 1)
    (if (>= (Variables|/Game/ThirdPerson/Blueprints/BP_ThirdPersonCharacter.BP_ThirdPersonCharacter_C|GetGold _asbp_third_person_character) (Variables|Default|GetExtractionCost))
      (Variables|/Game/ThirdPerson/Blueprints/BP_ThirdPersonCharacter.BP_ThirdPersonCharacter_C|SetGold _asbp_third_person_character (- (Variables|/Game/ThirdPerson/Blueprints/BP_ThirdPersonCharacter.BP_ThirdPersonCharacter_C|GetGold _asbp_third_person_character) (Variables|Default|GetExtractionCost)))
      (Default|ShowResult _asbp_third_person_character "直升机撤离成功，欢迎回家")
      (else
        (Development|PrintString "需要支付50金币启动直升机撤离")))
    (else
      (Default|ShowResult _asbp_third_person_character "海口撤离成功，欢迎回家"))))

(event Collision|EventActorBeginOverlap
  (params (OtherActor :type Actor%20Object%20Reference)))

(event EventTick
  (params (DeltaSeconds :type Float%20%28single-precision%29)))

(event EventBeginPlay
  (Rendering|SetActorHiddenInGame true)
  (Collision|SetActorEnableCollision false))

(fn ConstructionScript)

(fn ShowExitDoor
  (Rendering|SetActorHiddenInGame false)
  (Collision|SetActorEnableCollision true)
  (Development|PrintString "Exit Door SPawned"))