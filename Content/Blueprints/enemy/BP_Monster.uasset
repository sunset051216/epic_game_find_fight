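; BP_Monster is an enemy that detects the player, takes damage and rewards its killer.
; DetectSphere overlaps set or clear HasTarget in the BP_MonsterAIController blackboard, also storing target actor and location on entry.
; While HasTarget is true, Tick refreshes TargetLocation from player 0's position.
; TakeMonsterDamage lowers Health; on death it grants the attacker gold, a kill and combat power, then destroys the monster.
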(event OnComponentBeginOverlap(DetectSphere)
  (params (OverlappedComponent :type Primitive%20Component%20Object%20Reference) (OtherActor :type Actor%20Object%20Reference) (OtherComp :type Primitive%20Component%20Object%20Reference) (OtherBodyIndex :type Integer) (bFromSweep :type Boolean) (SweepResult :type Hit%20Result%20Structure%20%28by%20ref%29))
  (bind _asbp_third_person_character (Utilities|Casting|CastToBP_ThirdPersonCharacter OtherActor))
  (bind _asbp_monster_aicontroller (Utilities|Casting|CastToBP_MonsterAIController (Pawn|GetController self)))
  (AI|Components|Blackboard|SetValueasBool (AI|GetBlackboard _asbp_monster_aicontroller) (Utilities|Name|MakeLiteralName "HasTarget") true)
  (AI|Components|Blackboard|SetValueasObject (AI|GetBlackboard _asbp_monster_aicontroller) (Utilities|Name|MakeLiteralName "TargetActor") _asbp_third_person_character)
  (AI|Components|Blackboard|SetValueasVector (AI|GetBlackboard _asbp_monster_aicontroller) (Utilities|Name|MakeLiteralName "TargetLocation") (Transformation|GetActorLocation _asbp_third_person_character)))

(event OnComponentEndOverlap(DetectSphere)
  (params (OverlappedComponent :type Primitive%20Component%20Object%20Reference) (OtherActor :type Actor%20Object%20Reference) (OtherComp :type Primitive%20Component%20Object%20Reference) (OtherBodyIndex :type Integer))
  (Utilities|Casting|CastToBP_ThirdPersonCharacter OtherActor)
  (bind _asbp_monster_aicontroller (Utilities|Casting|CastToBP_MonsterAIController (Pawn|GetController self)))
  (AI|Components|Blackboard|SetValueasBool (AI|GetBlackboard _asbp_monster_aicontroller) (Utilities|Name|MakeLiteralName "HasTarget") false))

(event EventBeginPlay)

(event Collision|EventActorBeginOverlap
  (params (OtherActor :type Actor%20Object%20Reference)))

(event EventTick
  (params (DeltaSeconds :type Float%20%28single-precision%29))
  (bind _asbp_monster_aicontroller (Utilities|Casting|CastToBP_MonsterAIController (Pawn|GetController self)))
  (if (ScalableFloat|GetValueasBool (AI|GetBlackboard _asbp_monster_aicontroller) (Utilities|Name|MakeLiteralName "HasTarget"))
    (bind _asbp_third_person_character (Utilities|Casting|CastToBP_ThirdPersonCharacter (Game|GetPlayerCharacter 0)))
    (AI|Components|Blackboard|SetValueasVector (AI|GetBlackboard _asbp_monster_aicontroller) (Utilities|Name|MakeLiteralName "TargetLocation") (Transformation|GetActorLocation _asbp_third_person_character))))

(fn ConstructionScript)

(fn TakeMonsterDamage
  (params (DamageAmount :type Float%20%28double-precision%29) (Attacker :type BP%20Third%20Person%20Character%20Object%20Reference))
  (if (not (Variables|Default|GetbDead))
    (Variables|Default|SetHealth (- (Variables|Default|GetHealth) DamageAmount))
    (if (<= (Variables|Default|GetHealth) 0.0)
      (Variables|Default|SetbDead true)
      (Default|AddGold Attacker (Class|KismetMathLibrary|ToInt64(Float) (Variables|Default|GetRewardGold)))
      (Default|AddKillCount Attacker)
      (Variables|/Game/ThirdPerson/Blueprints/BP_ThirdPersonCharacter.BP_ThirdPersonCharacter_C|SetCombatPower Attacker (+ (Variables|/Game/ThirdPerson/Blueprints/BP_ThirdPersonCharacter.BP_ThirdPersonCharacter_C|GetCombatPower Attacker) 1))
      (Actor|DestroyActor)
      (Development|PrintString "Monster Dead"))))